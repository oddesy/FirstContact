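; Colony actor that tracks economy stats and opens a ColonyWidget UI when clicked.
; BeginPlay enables click events on the player controller, and each Sphere click creates a new widget and adds it to the viewport without passing it colony data.
; Tick calls UpdateColonyStats, which rebuilds the ColonyInfo struct with EconValue slightly more than doubled every frame, so growth is exponential and framerate-dependent.
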(event `self.ReceiveBeginPlay`
  (set `PlayerController.bEnableClickEvents` true (`GameplayStatics.GetPlayerController` 0)))

(event `self.Sphere.OnClicked`
  (params (TouchedComponent :type "PrimitiveComponent Object Reference") (ButtonPressed :type "Key Structure"))
  (bind _returnvalue (`|CreateWidget` "/Game/Colony/colonyWidget.colonyWidget_C"))
  (`UserWidget.AddToViewport` _returnvalue 0))

(event `self.ReceiveTick`
  (params (DeltaSeconds :type "Float (single-precision)"))
  (`self.Update Colony Stats`))

(fn `Update Colony Stats`
  (set `self.Colony Info` (make `/Game/Colony/colony_stats` 10.0 10.0 10.0 10.0 10.0 10.0 10.0 (* (`.econValue_24_F087B31649EDD47C25B165826E8D216A` (break `/Game/Colony/colony_stats` (`self.Colony Info`))) 2.01))))

(fn `UserConstructionScript`)